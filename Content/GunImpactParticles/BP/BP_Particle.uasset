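; BP_Particle is an actor that replays a chosen particle effect at its own position, in the gun impact particles content.
; On BeginPlay it spawns the Particle Niagara system at its scene root's location, then loops through a one-second Delay to spawn it again indefinitely.
; An alternative path that adds a Niagara component and a camera-relative transform calculation are left unconnected.
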(event `self.ReceiveBeginPlay`
  (`NiagaraFunctionLibrary.SpawnSystemAtLocation` (`self.Particle`) (`SceneComponent.K2_GetComponentLocation` (`self.DefaultSceneRoot`)) :!label _label)
  (`KismetSystemLibrary.Delay` 1.0)
  (goto _label))

(fn `UserConstructionScript`)